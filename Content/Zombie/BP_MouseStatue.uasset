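; BP_MouseStatue is a destructible statue actor that first-person projectiles can destroy.
; When a BP_FirstPersonProjectile overlaps its Capsule, the statue loses a fixed amount of health and the projectile is destroyed.
; Tick checks StatueHealth every frame and destroys the statue once it reaches zero or below.
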(event `self.Capsule.OnComponentBeginOverlap`
  (params (OverlappedComponent :type "PrimitiveComponent Object Reference") (OtherActor :type "Actor Object Reference") (OtherComp :type "PrimitiveComponent Object Reference") (OtherBodyIndex :type Integer) (bFromSweep :type Boolean) (SweepResult :type "HitResult Structure (by ref)"))
  (bind _asbp_first_person_projectile (cast `/Game/FirstPerson/Blueprints/BP_FirstPersonProjectile` OtherActor))
  (if true
    (set `self.StatueHealth` (- (`self.StatueHealth`) 200.0))
    (`self.K2_DestroyActor` _asbp_first_person_projectile)))

(event `self.ReceiveTick`
  (params (DeltaSeconds :type "Float (single-precision)"))
  (if (<= (`self.StatueHealth`) 0.0)
    (`self.K2_DestroyActor`)))

(fn `UserConstructionScript`)