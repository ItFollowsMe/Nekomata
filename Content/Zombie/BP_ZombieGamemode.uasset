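; BP_ZombieGamemode is a zombie wave game mode that starts spawning when play begins.
; StartGame calls SpawnZombies, which sets the total and remaining counts to five times the current wave.
; An empty loop precedes one that spawns BP_Zombie for half the total at SpawnLocation2.
; The SpawnLocation1 branch for the other half is disconnected, and nothing here advances waves.
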(event `self.ReceiveBeginPlay`
  (`self.Start Game`))

(event `Start Game`
  (`self.SpawnZombies`))

(event `SpawnZombies`
  (bind _output_get (set `self.ZombieTotal` (* (`self.CurrentWave`) 5)))
  (set `self.ZombiesLeft` _output_get)
  (for _index (range (+ _output_get 1))
    _)
  (for _ (range 1 (+ (/ (`self.ZombieTotal`) 2) 1))
    (`|SpawnActorFromClass` "/Game/Zombie/BP_Zombie.BP_Zombie_C" (`self.SpawnLocation2`) "Undefined" "MultiplyWithRoot" null null)))

(fn `UserConstructionScript`)